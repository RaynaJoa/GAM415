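; Portal actor that teleports actors entering its Trigger to the Box transform of its linked OtherPortal.
; The overlap also zeroes player zero's velocity and resets character and controller yaw, whichever actor entered.
; The construction script positions the Trigger and picks vortex material and Niagara effect by PortalVisual, clearing both without a valid ExitPartnerActor.
; TeleportToPortal is an unfinished tag lookup that never teleports.
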(event OnComponentBeginOverlap(trigger)
  (params (OverlappedComponent :type Primitive%20Component%20Object%20Reference) (OtherActor :type Actor%20Object%20Reference) (OtherComp :type Primitive%20Component%20Object%20Reference) (OtherBodyIndex :type Integer) (bFromSweep :type Boolean) (SweepResult :type Hit%20Result%20Structure%20%28by%20ref%29))
  (bind _returnvalue (Game|GetPlayerCharacter 0))
  (bind _otherportal (Variables|Default|GetOtherPortal))
  (bind _box (Variables|Portal_BP_C|GetBox _otherportal))
  (bind _returnvalue_2 (Transformation|GetWorldTransform _box))
  (Transformation|SetWorldTransform (Variables|/Script/Engine.Actor|GetRootComponent OtherActor) (Math|Transform|MakeTransform (.location _returnvalue_2) (.rotation _returnvalue_2) (.scale _returnvalue_2)) false true)
  (Pawn|SetControlRotation (Game|GetPlayerController 0) (Math|Rotator|MakeRotator 0.0 0.0 (+ (.yaw (Transformation|GetActorRotation (Game|GetPlayerCharacter 0))) 1.8e+02)))
  (Variables|/Script/Engine.MovementComponent|SetVelocity (Variables|/Script/Engine.Character|GetCharacterMovement _returnvalue) "0, 0, 0")
  (Transformation|SetActorRotation _returnvalue (Math|Rotator|MakeRotator 0.0 0.0 (+ (.yaw (Transformation|GetActorRotation (Variables|Default|GetOtherPortal))) 1.8e+02))))

(event OnComponentBeginOverlap(Box)
  (params (OverlappedComponent :type Primitive%20Component%20Object%20Reference) (OtherActor :type Actor%20Object%20Reference) (OtherComp :type Primitive%20Component%20Object%20Reference) (OtherBodyIndex :type Integer) (bFromSweep :type Boolean) (SweepResult :type Hit%20Result%20Structure%20%28by%20ref%29)))

(event EventBeginPlay)

(event Collision|EventActorBeginOverlap
  (params (OtherActor :type Actor%20Object%20Reference)))

(event EventTick
  (params (DeltaSeconds :type Float%20%28single-precision%29)))

(fn ConstructionScript
  (bind _plane (Variables|Default|GetPlane))
  (bind _ns_portal (Variables|Default|GetNS_Portal))
  ;[1 1 1] Setting up colors for different portals
  (Transformation|SetRelativeLocation (Variables|Default|Gettrigger) (Variables|Setup|GetCOL%20Sohere%20Location) false false)
  (switch Utilities|FlowControl|Switch|SwitchonEnum_GateSkin (Variables|Setup|GetPortal%20Visual)
    (:NewEnumerator0
      (Rendering|Material|SetMaterial _plane 0 "/Game/Materials/MAT_Vortex_Blue.MAT_Vortex_Blue")
      (Class|NiagaraComponent|SetAsset _ns_portal "/Game/Materials/VFX/NS_Portal.NS_Portal" true))
    (:NewEnumerator1
      (Rendering|Material|SetMaterial _plane 0 "/Game/Materials/MAT_Vortex_Red.MAT_Vortex_Red")
      (Class|NiagaraComponent|SetAsset _ns_portal "/Game/Materials/VFX/NS_Portal_Red.NS_Portal_Red" true))
    (:NewEnumerator2
      (Rendering|Material|SetMaterial _plane 0 "/Game/Materials/MAT_Vortex_Yellow.MAT_Vortex_Yellow")
      (Class|NiagaraComponent|SetAsset _ns_portal "/Game/Materials/VFX/NS_Portal_Yellow.NS_Portal_Yellow" true)))
  (Utilities|IsValid (Variables|Teleport|GetExitPartnerActor)
    (:Is%20Not%20Valid
      (Rendering|Material|SetMaterial (Variables|Default|GetPlane) 0 0)
      (Class|NiagaraComponent|SetAsset (Variables|Default|GetNS_Portal) 0 true))))

(fn TeleporttoPortal
  (params (NewParam :type BP%20First%20Person%20Character%20Object%20Reference))
  (bind _outactors (Actor|GetAllActorsOfClasswithTag "Portal_BP_C" (Variables|Default|GetPortalColor)))
  (LocalVariables|SetPortal (Utilities|Array|Get(acopy) _outactors))
  (Utilities|IsValid (Utilities|Array|Get(acopy) _outactors)
    (:Is%20Not%20Valid
      (Development|PrintText "nah"))))